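; EnemyAI is an AI controller that sends its enemy pawn in a straight line along the X axis to a destination supplied by the game mode.
; On the first Tick it sets a one-shot flag, gets the destination X from GameModeBP and keeps the pawn's current Y and Z.
; It then issues a single MoveToLocation with pathfinding disabled.
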(event EventBeginPlay)

(event EventTick
  (params (DeltaSeconds :type Float%20%28single-precision%29))
  (bind _self self)
  (bind _returnvalue (Pawn|GetControlledPawn _self))
  (bind _returnvalue_2 (Transformation|GetActorLocation _returnvalue))
  (bind (_x _y _z) (Math|Vector|BreakVector _returnvalue_2))
  (if (not (Variables|Default|GetTargetSet))
    (Variables|Default|SetTargetSet true)
    (bind _asgame_mode_bp (Utilities|Casting|CastToGameModeBP (Game|GetGameMode)))
    (bind _returnvalue_3 (Class|BasicGameModeBase|GetEnemyDestPosition _asgame_mode_bp))
    (bind _output_get (Variables|Default|SetTarget (Math|Vector|MakeVector _returnvalue_3 _y _z)))
    (AI|Navigation|MovetoLocation _output_get -1.0 true false false true 0)))

(fn ConstructionScript)